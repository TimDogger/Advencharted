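; BP_Cube is an inspectable toy cube item, presented in Russian as a children's cube with a long promotional description.
; On BeginPlay it writes random RGB values into the first three custom primitive data slots of each of its primitive components, giving per-component color data without dynamic material instances.
; Getter functions supply the IDDA_Inspect interaction definition, item name and description.
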(event `self.ReceiveBeginPlay`
  (bind (_returnvalue_r _returnvalue_g _returnvalue_b) (break `LinearColor` (`KismetMathLibrary.MakeColor` (`KismetMathLibrary.RandomFloatInRange` 0.0 1.0) (`KismetMathLibrary.RandomFloatInRange` 0.0 1.0) (`KismetMathLibrary.RandomFloatInRange` 0.0 1.0))))
  (for _array_element (`self.K2_GetComponentsByClass` "/Script/Engine.PrimitiveComponent")
    (`PrimitiveComponent.SetCustomPrimitiveDataFloat` _array_element 0 _returnvalue_r)
    (`PrimitiveComponent.SetCustomPrimitiveDataFloat` _array_element 1 _returnvalue_g)
    (`PrimitiveComponent.SetCustomPrimitiveDataFloat` _array_element 2 _returnvalue_b)))

(fn `GetInteractionDefinition`
  (returns (ReturnValue :type "InteractionDefinition Object Reference"))
  (return "/Game/Interactions/DataAssets/IDDA_Inspect.IDDA_Inspect"))

(fn `GetItemDescription`
  (returns (ReturnValue :type Text))
  (return "\"Детский кубик\" - это не просто игрушка, это мир, полный открытий и возможностей для вашего ребенка. Этот яркий и привлекательный предмет является символом беззаботного детства и радости открытия нового. Каждая сторона кубика украшена различными геометрическими фигурами и цветами, способствующими развитию визуального восприятия и координации движений.  Кубик может стать отличным способом провести время, развивая логическое мышление и воображение. Он изготовлен из безопасных материалов, что делает его идеальным для маленьких детей. \"Детский кубик\" - это не просто игрушка, это ключ к миру обучения и развития через игру.  Каждая сторона кубика предлагает новые возможности для обучения и развлечения. От простых геометрических форм и цветов до более сложных пазлов и задач, этот кубик предлагает бесконечные возможности для обучения и развития.  Кубик легко удерживать в руках, и его можно использовать для различных игр и упражнений. Он может помочь развить моторику, координацию и баланс, а также стимулировать воображение и творческое мышление.  \"Детский кубик\" - это отличный подарок для любого ребенка. Он предлагает бесконечные возможности для обучения и развлечения, а также помогает развивать важные навыки и способности. Этот кубик - это не просто игрушка, это инструмент для обучения, который поможет вашему ребенку расти и развиваться.  В конце концов, \"Детский кубик\" - это не просто игрушка, это возможность для вашего ребенка открыть для себя мир вокруг себя. Он помогает развивать важные навыки и способности, а также предлагает бесконечные возможности для обучения и развлечения. \"Детский кубик\" - это подарок, который продолжает дарить."))

(fn `GetItemName`
  (returns (ReturnValue :type Text))
  (return "Кубик "))

(fn `UserConstructionScript`)