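; BP_Sphere is an interactable sphere that glows when ready to interact and reacts physically when used.
; A Glow timeline drives the "Glow" material parameter, reversing when the sphere stops being ready.
; Interacting launches the sphere upward with a random velocity-change impulse and randomizes the hit component's scale per axis.
; It supplies IDDA_RandomColor as its interaction definition, while GetInteractableComponent returns no component.
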(event `self.OnReadyToInteract`
  (params (Interactor :type "Actor Object Reference") (HitComponent :type "PrimitiveComponent Object Reference"))
  (bind (_direction _glowanim) (`Timeline|Glow` :!label _label)
    (:`Update`
      (`MeshComponent.SetScalarParameterValueOnMaterials` (`self.Sphere`) "Glow" _glowanim))))

(event `self.OnNotReadyToInteract`
  (params (Interactor :type "Actor Object Reference") (HitComponent :type "PrimitiveComponent Object Reference"))
  (goto _label :!via `Reverse`))

(event `self.OnInteract`
  (params (Interactor :type "Actor Object Reference") (HitComponent :type "PrimitiveComponent Object Reference"))
  (bind _returnvalue (`KismetMathLibrary.RandomFloatInRange` 0.3 1.0))
  (`PrimitiveComponent.AddImpulse` (`self.Sphere`) (* (0.0 0.0 1.0) (`KismetMathLibrary.RandomFloatInRange` 50.0 300.0)) "None" true)
  (`SceneComponent.SetWorldScale3D` HitComponent (`KismetMathLibrary.MakeVector` _returnvalue _returnvalue _returnvalue)))

(fn `GetInteractableComponent`
  (returns (ReturnValue :type "PrimitiveComponent Object Reference"))
  (return null))

(fn `GetInteractionDefinition`
  (returns (ReturnValue :type "InteractionDefinition Object Reference"))
  (return "/Game/Interactions/DataAssets/IDDA_RandomColor.IDDA_RandomColor"))

(fn `UserConstructionScript`)