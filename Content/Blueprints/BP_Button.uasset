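; BP_Button is an interactable button that relays an interaction to every BP_Sphere in the world.
; On interact it plays a click sound, then calls OnInteract on each sphere with itself as Interactor.
; It also fires each sphere's interaction definition with the original Interactor.
; It reports Cube1's world location as its interactable location and leaves its component and definition getters empty.
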(event `self.OnInteract`
  (params (Interactor :type "Actor Object Reference") (HitComponent :type "PrimitiveComponent Object Reference"))
  (`GameplayStatics.PlaySound2D` "/Engine/VREditor/Sounds/UI/Click_on_Button.Click_on_Button" 1.0 1.0 0.0 null null)
  (bind _outactors (`GameplayStatics.GetAllActorsOfClass` "/Game/Blueprints/BP_Sphere.BP_Sphere_C"))
  (for _array_element _outactors
    (`Interactable.OnInteract` _array_element self (`self.GetComponentByClass` _array_element "/Script/Engine.PrimitiveComponent"))
    (`InteractionDefinition.OnInteract` (`AdvenchartedLibrary.GetInteractionDefinitionForActor` _array_element) Interactor _array_element)))

(fn `GetInteractableComponent`
  (returns (ReturnValue :type "PrimitiveComponent Object Reference"))
  (return null))

(fn `GetInteractableLocation`
  (returns (bWorldLocation :type Boolean) (ReturnValue :type "Vector Structure"))
  (return true (`SceneComponent.K2_GetComponentLocation` (`self.Cube1`))))

(fn `GetInteractionDefinition`
  (returns (ReturnValue :type "InteractionDefinition Object Reference"))
  (return null))

(fn `UserConstructionScript`)